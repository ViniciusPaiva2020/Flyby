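; Refugee AI controller that starts the Refugiado_BT behavior tree on BeginPlay and feeds it sightings of pickups.
; Perception updates react only to container and medkit pickups, writing whether the pickup is sensed to the SeesPickup blackboard key.
; The matching component's world location, from either the container or the medkit, is written to PickupLocation on every update, including when sensing is lost.
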(event OnTargetPerceptionUpdated(AIPerception)
  (params (Actor :type Actor%20Object%20Reference) (Stimulus :type AI%20Stimulus%20Structure))
  (bind _returnvalue (AI|GetBlackboard 0))
  (bind _returnvalue_2 (Utilities|Name|MakeLiteralName "PickupLocation"))
  ;[1 1 1] checa o tipo de pickup
  (bind _ascontainer_pickup (Utilities|Casting|CastToContainerPickup Actor)
    (:then
      (Variables|Default|SetisContainer true))
    (:CastFailed
      (bind _asmedkit_pickup (Utilities|Casting|CastToMedkitPickup Actor))
      (Variables|Default|SetisContainer false)))
  ;[1 1 1] seta as variáveis da blackboard
  (AI|Components|Blackboard|SetValueasBool _returnvalue (Utilities|Name|MakeLiteralName "SeesPickup") (.bSuccessfullySensed (Utilities|Struct|BreakAIStimulus Stimulus)))
  (if (Variables|Default|GetisContainer)
    (AI|Components|Blackboard|SetValueasVector _returnvalue _returnvalue_2 (Transformation|GetWorldLocation (Variables|/Game/Blueprints/Objetivos/ContainerPickup.ContainerPickup_C|GetContainer _ascontainer_pickup)))
    (else
      (AI|Components|Blackboard|SetValueasVector _returnvalue _returnvalue_2 (Transformation|GetWorldLocation (Variables|/Game/Blueprints/Objetivos/MedkitPickup.MedkitPickup_C|GetKit_Medico _asmedkit_pickup))))))

(event EventBeginPlay
  ;[1 1 1] inicia a AI
  (AI|RunBehaviorTree "/Game/Blueprints/Refugiado_BT.Refugiado_BT"))

(fn ConstructionScript)