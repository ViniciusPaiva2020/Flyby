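; ContainerTarget is an objective drop zone that completes when a Drop_Item_2 actor overlaps it.
; A Finished flag guards against repeat completion, then the overlapping item is destroyed and ContainerObjectives on the FlybyInstance game instance is incremented and printed.
; It then spawns a ContainerPickup at its Arrow component's location, intended for AI use, and destroys itself.
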(event Collision|EventActorBeginOverlap
  (params (OtherActor :type Actor%20Object%20Reference))
  ;[1 1 1] colisão
  (if (not (Variables|Default|Getfinished))
    (Utilities|Casting|CastToDrop_Item_2 OtherActor)
    ;[1 1 1] impede o mesmo objetivo de ser completo várias vezes
    (Actor|DestroyActor OtherActor)
    (Variables|Default|Setfinished true)
    ;[1 1 1] aumenta variável de objetivos
    (bind _asflyby_instance (Utilities|Casting|CastToFlybyInstance (Game|GetGameInstance)))
    (bind _output_get (Variables|/Game/Blueprints/Objetivos/FlybyInstance.FlybyInstance_C|SetcontainerObjectives _asflyby_instance (+ (Variables|/Game/Blueprints/Objetivos/FlybyInstance.FlybyInstance_C|GetcontainerObjectives _asflyby_instance) 1)))
    (Development|PrintString (Utilities|String|ToString(Integer) _output_get))
    ;[1 1 1] cria um pickup pra AI usar
    (Game|SpawnActorfromClass "/Game/Blueprints/Objetivos/ContainerPickup.ContainerPickup_C" (Math|Transform|MakeTransform (Transformation|GetWorldLocation (Variables|Default|GetArrow))) "Undefined" 0 0)
    (Actor|DestroyActor)))

(fn ConstructionScript)

(fn NewFunction0
  (return false))